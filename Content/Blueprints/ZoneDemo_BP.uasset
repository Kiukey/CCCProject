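; ZoneDemo_BP is a demo proximity zone that switches cameras depending on how close the Erika actor is to it.
; On BeginPlay it takes the CameraManager from GameModeManager_BP.
; Every tick it measures Erika's distance to itself, enabling the "Other" camera within a small fixed radius and the "Erika" camera otherwise.
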(event EventBeginPlay
  (bind _asgame_mode_manager_bp (Utilities|Casting|CastToGameModeManager_BP (Game|GetGameMode)))
  (Variables|Default|SetCamera%20Manager (Variables|/Script/CCCProject.GameModeManager|GetcameraManager _asgame_mode_manager_bp)))

(event EventTick
  (params (DeltaSeconds :type Float%20%28single-precision%29))
  (bind _erika (Variables|Default|GetErika)
    (:then
      (if (< (Math|Vector|Distance(Vector) (Transformation|GetActorLocation _erika) (Transformation|GetActorLocation)) 1e+02)
        (bind _camera_manager (Variables|Default|GetCamera%20Manager)
          (:then
            (Class|CameraManager|Enable _camera_manager "Other"))
          (:else))
        (else
          (bind _camera_manager_2 (Variables|Default|GetCamera%20Manager)
            (:then
              (Class|CameraManager|Enable _camera_manager_2 "Erika"))
            (:else)))))
    (:else)))

(fn ConstructionScript)